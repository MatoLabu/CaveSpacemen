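; BP_Tree_01 is a flammable tree that catches fire, spreads it to nearby trees and ends up charred.
; Inflame runs once, notifies JetpackGameMode and attaches a scaled BP_Flame at the flame anchor.
; After a short delay it calls Inflame on unburnt BP_Tree_Parent trees overlapping ChainFlameColl through TreeColl-tagged components, creating a chain reaction.
; Meanwhile a timeline times the burn, then IsCalcinated removes the flame and swaps trunk and branch materials.
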(event `Inflame`
  (bind _treeflameanchor (`self.TreeFlameAnchor`))
  ;[1 1 1] Si pas déjà enflammé
  (if (not (`self.IsInflamed`))
    (set `self.IsInflamed` true)
    ;[1 1 1] Lance les conséquences gameplay
    (bind _asjetpack_game_mode (cast `/Game/JetpackGameMode` (`GameplayStatics.GetGameMode`)))
    (`/Game/JetpackGameMode.InflameATree` _asjetpack_game_mode)
    (`|ExecutionSequence`
      (:`then_0`
        ;[1 1 1] Add flame fx
        (bind _returnvalue (`|SpawnActorFromClass` "/Game/Fireboxes/BP_Flame.BP_Flame_C" (`SceneComponent.K2_GetComponentToWorld` _treeflameanchor) "Undefined" "OverrideRootScale"))
        (`self.SetActorScale3D` _returnvalue (7.0 7.0 7.0))
        (`self.K2_AttachToComponent` _returnvalue _treeflameanchor "None" "KeepWorld" "KeepWorld" "KeepRelative" true)
        (set `self.TreeFlames` _returnvalue)
        (`KismetSystemLibrary.Delay` 0.5)
        ;[1 1 1] infects other trees
        (for _array_element (`PrimitiveComponent.GetOverlappingComponents` (`self.ChainFlameColl`))
          (`KismetSystemLibrary.PrintString` (`KismetStringLibrary.Concat_StrStr` "Component: " (`KismetSystemLibrary.GetDisplayName` _array_element)))
          (if (`ActorComponent.ComponentHasTag` _array_element "TreeColl")
            (`KismetSystemLibrary.PrintString` "Touched the TreeColl" true true (struct :`G` 1.0 :`B` 0.17924 :`A` 1.0))
            (bind _asbp_tree_parent (cast `/Game/Trees/BP_Tree_Parent` (`ActorComponent.GetOwner` _array_element))
              (:`then`
                (`KismetSystemLibrary.PrintString` (`KismetStringLibrary.Concat_StrStr` "Owner is:" (`KismetSystemLibrary.GetDisplayName` _asbp_tree_parent)) true true (struct :`G` 0.200821 :`B` 1.0 :`A` 1.0))
                (if (not (`/Game/Trees/BP_Tree_Parent.IsInflamed` _asbp_tree_parent))
                  (`KismetSystemLibrary.PrintString` "Is not inflamed, BURN BABY BURN!!!!")
                  (`self.Inflame` _asbp_tree_parent)
                  (else
                    (`KismetSystemLibrary.PrintString` "Is AllReady Inflamed..."))))
              (:`CastFailed`
                (`KismetSystemLibrary.PrintString` "The Owner is not a Tree_Parent" true true (struct :`R` 0.952595 :`G` 1.0 :`A` 1.0))))
            (else
              (`KismetSystemLibrary.PrintString` "Touched a component, but it's not a TreeColl" true true (struct :`R` 1.0 :`B` 0.0077 :`A` 1.0))))))
      (:`then_1`
        ;[1 1 1] After burning, set tree to calcinated
        (`TimelineComponent.SetTimelineLength` (`self.TreeInflamed`) 5.0)
        (`Timeline|TreeInflamed` :!via `PlayFromStart`
          (:`Finished`
            (`self.IsCalcinated`)))))))

(event `IsCalcinated`
  (bind _sapin1 (`self.sapin1`))
  ;[1 1 1] Remove flame fx
  (`self.SetLifeSpan` (`self.TreeFlames`) 0.01)
  (`PrimitiveComponent.SetMaterial` _sapin1 0 "/Game/Trees/M_trunk2.M_trunk2")
  (`PrimitiveComponent.SetMaterial` _sapin1 1 "/Game/Trees/M_branch2.M_branch2"))

(fn `UserConstructionScript`)