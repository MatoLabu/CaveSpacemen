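; BP_PlanetGod is a planet actor that keeps its Scene component oriented to the level's sun.
; Construction caches the first DirectionalLight found as Sun, then SetCircleRot copies that light's world rotation onto Scene, repeating every Tick.
; An AddShafts helper spawns and attaches particle system components in a loop but is not called here, and a camera-facing rotation toward the caveman pawn is left disconnected.
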(event `self.ReceiveTick`
  (params (DeltaSeconds :type "Float (single-precision)"))
  (`self.SetCircleRot`))

(fn `add shafts`
  (params (`Shaft number` :type Integer) (`Planet size` :type "Float (double-precision)"))
  (for _ (range (+ `Shaft number` 1))
    (bind _returnvalue (`AddComponent|Particle System Component_0`))
    (`SceneComponent.K2_AttachToComponent` _returnvalue null "None" "KeepRelative" "KeepRelative" "KeepRelative" true)))

(fn `SetCircleRot`
  (`SceneComponent.K2_SetWorldRotation` (`self.Scene`) (`SceneComponent.K2_GetComponentRotation` (`Light.LightComponent` (`self.Sun`))) false false))

(fn `UserConstructionScript`
  (bind _outactors (`GameplayStatics.GetAllActorsOfClass` "/Script/Engine.DirectionalLight"))
  (set `self.Sun` (`KismetArrayLibrary.Array_Get` _outactors))
  (`self.SetCircleRot`))