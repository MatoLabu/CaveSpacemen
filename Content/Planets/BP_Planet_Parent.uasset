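; BP_Planet_Parent is a planet Blueprint, named as a parent class, that sets up the planet's visual component.
; Its construction script sets the relative scale of PlanetVisual to a fixed, uniform enlargement.
; The remaining nodes are disconnected debug leftovers that test casts to physics constraint, spring and thruster components or print a child component's name, and never run.
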(fn `UserConstructionScript`
  (`SceneComponent.SetRelativeScale3D` (`self.PlanetVisual`) (3.0 3.0 3.0)))