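; HUD manager actor that runs the caveman jetpack game's round flow, from title fade and 3-2-1 countdown to end screen.
; After the countdown it enables pawn input and drives the game clock from a timeline update, formatted as minutes:seconds:hundredths.
; When GameOver is set, including on timeout, it notifies the pawn and all planets.
; JetpackGameMode's FireboxCounter being above zero selects victory over failure text and audio.
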(event `self.ReceiveBeginPlay`
  (bind _hud_ref (`self.HUD_Ref`))
  ;[1 1 1] INIT
  (bind _returnvalue (`|CreateWidget` "/Game/HUD/W_HUD.W_HUD_C"))
  (bind _output_get (set `self.HUD_Ref` _returnvalue))
  (`UserWidget.AddToViewport` _output_get 0)
  (`self.FormatGameCountdownForHUD`)
  (`KismetSystemLibrary.Delay` 4.0)
  (`Widget.SetVisibility` (`/Game/HUD/W_HUD.TITLE` _hud_ref) "Hidden")
  (`UserWidget.PlayAnimation` _hud_ref (`/Game/HUD/W_HUD.TitleFade` _hud_ref) 0.0 1 "Forward")
  (`KismetSystemLibrary.Delay` 1.0)
  (`self.StartCountdown`))

(event `StartCountdown`
  (bind _hud_ref (`self.HUD_Ref`))
  (bind _hud_ref_2 (`self.HUD_Ref`))
  (bind _hud_ref_3 (`self.HUD_Ref`))
  (bind _hud_ref_4 (`self.HUD_Ref`))
  (bind _hud_ref_5 (`self.HUD_Ref`))
  (bind _hud_ref_6 (`self.HUD_Ref`))
  (bind _startcountdown (`/Game/HUD/W_HUD.StartCountdown` _hud_ref_6))
  (bind _returnvalue (> (`/Game/JetpackGameMode.FireboxCounter` (cast `/Game/JetpackGameMode` (`GameplayStatics.GetGameMode`) :!pure true)) 0))
  (`self.SetTextAndFontSizeAndAnim` (`/Game/HUD/W_HUD.StartCountdown` _hud_ref_3) "3" 150 _hud_ref_3)
  (`FMODBlueprintStatics.PlayEvent2D` "/Game/FMOD/Events/Begin.Begin")
  (`KismetSystemLibrary.Delay` 1.0)
  (`self.SetTextAndFontSizeAndAnim` (`/Game/HUD/W_HUD.StartCountdown` _hud_ref) "2" 150 _hud_ref)
  (`FMODBlueprintStatics.PlayEvent2D` "/Game/FMOD/Events/Begin.Begin")
  (`KismetSystemLibrary.Delay` 1.0)
  (`self.SetTextAndFontSizeAndAnim` (`/Game/HUD/W_HUD.StartCountdown` _hud_ref_4) "1" 150 _hud_ref_4)
  (`FMODBlueprintStatics.PlayEvent2D` "/Game/FMOD/Events/Begin.Begin")
  (`KismetSystemLibrary.Delay` 1.0)
  (`self.SetTextAndFontSizeAndAnim` (`/Game/HUD/W_HUD.StartCountdown` _hud_ref_5) "Burn all the fireplaces!\n\nDon't burn trees!" 30 _hud_ref_5)
  (`FMODBlueprintStatics.PlayEvent2D` "/Game/FMOD/Events/Grunt.Grunt")
  ;[1 1 1] Enable inputs
  (bind _asbp_pawn_caveman (cast `/Game/CharCaveman/BP_PawnCaveman` (`GameplayStatics.GetPlayerPawn` 0)))
  (set `/Game/CharCaveman/BP_PawnCaveman.GameIsOver` false _asbp_pawn_caveman)
  (`KismetSystemLibrary.Delay` 4.0)
  (`Widget.SetVisibility` (`/Game/HUD/W_HUD.StartCountdown` _hud_ref_2) "Hidden")
  (`Widget.SetVisibility` (`/Game/HUD/W_HUD.Counter` _hud_ref_2) "HitTestInvisible") ; Show counter
  (`Timeline|GameTimer`
    (:`Update`
      (if (not (`self.GameOver`))
        (`|ExecutionSequence`
          (:`then_0`
            (bind _output_get (set `self.GameCountdown` (- (`self.GameCountdown`) (`GameplayStatics.GetWorldDeltaSeconds`))))
            (if (<= _output_get 0.0)
              (set `self.GameCountdown` 0.0)
              (set `self.GameOver` true)))
          (:`then_1`
            (`self.FormatGameCountdownForHUD`)))
        (else
          (`TimelineComponent.Stop` (`self.GameTimer`))
          (`Widget.SetVisibility` _startcountdown "HitTestInvisible")
          (`self.SetTextAndFontSizeAndAnim` _startcountdown (select `bool` _returnvalue :`false` "GAME OVER... TRY AGAIN!" :`true` "GOOD JOB SPACECAVEMAN!" :!type "Text") 80)
          (`Widget.SetVisibility` (`/Game/HUD/W_HUD.Restart` _hud_ref_6) "Visible")
          (`|ExecutionSequence`
            (:`then_0`
              (bind _asbp_pawn_caveman_2 (cast `/Game/CharCaveman/BP_PawnCaveman` (`GameplayStatics.GetPlayerPawn` 0)))
              (`/Game/CharCaveman/BP_PawnCaveman.GameOver` _asbp_pawn_caveman_2))
            (:`then_1`
              (bind _outactors (`GameplayStatics.GetAllActorsOfClass` "/Game/Planets/BP_Planet_Parent.BP_Planet_Parent_C"))
              (for _array_element _outactors
                (`/Game/Planets/BP_Planet_Parent.GameOver` _array_element)))
            (:`then_2`
              (if _returnvalue
                (`FMODBlueprintStatics.PlayEvent2D` "/Game/FMOD/Events/MusicVictory.MusicVictory")
                (`KismetSystemLibrary.Delay` 3.0)
                (`Widget.SetVisibility` (`/Game/HUD/W_HUD.WIN` (`self.HUD_Ref`)) "Visible")
                (`FMODBlueprintStatics.PlayEvent2D` "/Game/FMOD/Events/MusicVictory.MusicVictory")
                (else
                  (`FMODBlueprintStatics.PlayEvent2D` "/Game/FMOD/Events/Loose.Loose"))))))))))

(fn `FormatGameCountdownForHUD`
  (bind _gamecountdown (`self.GameCountdown`))
  (set `self.GameCountdown_ForHUD` (`|FormatText` "{Minutes}:{Seconds}:{Milliseconds}" (`KismetTextLibrary.Conv_IntToText` (`KismetMathLibrary.FTrunc` (/ _gamecountdown 60.0)) true 1 2) (`KismetTextLibrary.Conv_IntToText` (`KismetMathLibrary.FTrunc` (mod _gamecountdown 60.0)) true 2 2) (`KismetTextLibrary.Conv_IntToText` (`KismetMathLibrary.FTrunc` (* (- _gamecountdown (`KismetMathLibrary.Conv_IntToDouble` (`KismetMathLibrary.FTrunc` _gamecountdown))) 100.0)) true 2 2)))
  (return))

(fn `SetTextAndFontSizeAndAnim`
  (params (Text :type "TextBlock Object Reference") (TextValue :type Text) (FontSise :type Integer) (HUDRef :type "/Game/HUD/W_HUD Object Reference"))
  (bind (_font_fontobject _font_fontmaterial _font_typefacefontname) (break `SlateFontInfo` (`TextBlock.Font` Text)))
  (`TextBlock.SetText` Text TextValue)
  (`TextBlock.SetFont` Text (make `SlateFontInfo` _font_fontobject _font_fontmaterial _font_typefacefontname FontSise))
  (`UserWidget.PlayAnimation` HUDRef (`/Game/HUD/W_HUD.CountdownBounce` HUDRef) 0.0 1 "Forward")
  (return))

(fn `UserConstructionScript`)