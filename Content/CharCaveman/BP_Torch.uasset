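; Caveman torch Blueprint that sets fireboxes and trees alight on contact.
; On BeginPlay its skeletal mesh loops an arm idle animation.
; A sphere overlap calls Inflame on any Firebox, or on a Tree only when the overlapped component carries the TreeColl tag.
; Two self-restarting, random-length timelines for spinning four fire components are present but disconnected, so they never run.
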(event `self.ReceiveBeginPlay`
  (`SkeletalMeshComponent.PlayAnimation` (`self.SkeletalMesh`) "/Game/CharCaveman/ARM/Arm_idle_Anim.Arm_idle_Anim" true))

(event `self.Sphere.OnComponentBeginOverlap`
  (params (OverlappedComponent :type "PrimitiveComponent Object Reference") (OtherActor :type "Actor Object Reference") (OtherComp :type "PrimitiveComponent Object Reference") (OtherBodyIndex :type Integer) (bFromSweep :type Boolean) (SweepResult :type "HitResult Structure (by ref)"))
  (bind _asbp_firebox_parent (cast `/Game/Fireboxes/BP_Firebox_Parent` OtherActor) ; test if Firebox
    (:`then`
      (`/Game/Fireboxes/BP_Firebox_Parent.Inflame` _asbp_firebox_parent))
    (:`CastFailed`
      (bind _asbp_tree_parent (cast `/Game/Trees/BP_Tree_Parent` OtherActor))
      (if (`ActorComponent.ComponentHasTag` OtherComp "TreeColl")
        (`/Game/Trees/BP_Tree_Parent.Inflame` _asbp_tree_parent)))))

(fn `UserConstructionScript`)