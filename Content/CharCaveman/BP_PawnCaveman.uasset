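; Player pawn for a caveman flying by jetpack: a physics sphere steered by look axes, with a tilting torch.
; Each jet input, gated by a game-over check, fires a burst impulse and camera shake, then a timeline applies continuous thrust until release.
; Tick plays ignition and steam sounds, scaling steam pitch with velocity.
; GameIsOver starts true at BeginPlay; GameOver sets it again and freezes the sphere through huge linear damping.
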(event `self.ReceiveBeginPlay`
  (set `self.GameIsOver` true)
  (bind (_direction _newtrack_0) (`Timeline|Timeline_4`)
    (:`Update`
      (`SceneComponent.K2_SetRelativeLocation` (`self.SM_Face`) (`KismetMathLibrary.MakeVector` _newtrack_0 0.0 2.0) false false))))

(event `InputAxis|LookLR`
  (params (AxisValue :type "Float (single-precision)"))
  (`SceneComponent.K2_AddLocalRotation` (`self.Sphere`) (`KismetMathLibrary.MakeRotator` 0.0 (stale `InputAxis|LookUD` AxisValue) AxisValue) false false :!label _label)
  (`SceneComponent.K2_SetRelativeRotation` (`self.Torch`) (`KismetMathLibrary.MakeRotator` (* (stale `InputAxis|LookUD` AxisValue) 1.0) 0.0 (* AxisValue -0.5)) false false))

(event `InputAxis|LookUD`
  (params (AxisValue :type "Float (single-precision)"))
  (goto _label))

(event `InputAction|JetForward`
  (params (Key :type "Key Structure" :default "AnyKey"))
  (bind _sphere (`self.Sphere`))
  (bind _returnvalue (* (`SceneComponent.GetForwardVector` _sphere) (* (`GameplayStatics.GetWorldDeltaSeconds`) (`self.Jetpack_Speed`))))
  (:`Pressed`
    (`self.TestIsGameIsNotOver`
      (:`TRUE`
        (set `self.InputFront` true)
        (`self.JetShake` false)
        (`PrimitiveComponent.AddImpulse` _sphere (* _returnvalue (`self.JetpackBurstForce`)) "None" false)
        (`Timeline|Timeline_0` :!label _label_2
          (:`Update`
            (`PrimitiveComponent.AddImpulse` _sphere _returnvalue "None" false))))))
  (:`Released`
    (`self.TestIsGameIsNotOver`
      (:`TRUE`
        (set `self.InputFront` false)
        (goto _label_2 :!via `Stop`)))))

(event `InputAction|JetBackward`
  (params (Key :type "Key Structure" :default "AnyKey"))
  (bind _sphere (`self.Sphere`))
  (bind _returnvalue (* (* (`SceneComponent.GetForwardVector` _sphere) (* (`GameplayStatics.GetWorldDeltaSeconds`) (`self.Jetpack_Speed`))) -1.0))
  (:`Pressed`
    (`self.TestIsGameIsNotOver`
      (:`TRUE`
        (set `self.InputBack` true)
        (`self.JetShake` false)
        (`PrimitiveComponent.AddImpulse` _sphere (* _returnvalue (`self.JetpackBurstForce`)) "None" false)
        (`Timeline|Timeline_1` :!label _label_3
          (:`Update`
            (`PrimitiveComponent.AddImpulse` _sphere _returnvalue "None" false))))))
  (:`Released`
    (`self.TestIsGameIsNotOver`
      (:`TRUE`
        (set `self.InputBack` false)
        (goto _label_3 :!via `Stop`)))))

(event `InputAction|JetLeft`
  (params (Key :type "Key Structure" :default "AnyKey"))
  (bind _sphere (`self.Sphere`))
  (bind _returnvalue (* (* (`SceneComponent.GetRightVector` _sphere) (* (`GameplayStatics.GetWorldDeltaSeconds`) (`self.Jetpack_Speed`))) -1.0))
  (:`Pressed`
    (`self.TestIsGameIsNotOver`
      (:`TRUE`
        (set `self.InputLeft` true)
        (`self.JetShake` true)
        (`PrimitiveComponent.AddImpulse` _sphere (* _returnvalue (`self.JetpackBurstForce`)) "None" false)
        (`Timeline|Timeline_2` :!label _label_4
          (:`Update`
            (`PrimitiveComponent.AddImpulse` _sphere _returnvalue "None" false))))))
  (:`Released`
    (`self.TestIsGameIsNotOver`
      (:`TRUE`
        (set `self.InputLeft` false)
        (goto _label_4 :!via `Stop`)))))

(event `InputAction|JetRight`
  (params (Key :type "Key Structure" :default "AnyKey"))
  (bind _sphere (`self.Sphere`))
  (bind _returnvalue (* (`SceneComponent.GetRightVector` _sphere) (* (`GameplayStatics.GetWorldDeltaSeconds`) (`self.Jetpack_Speed`))))
  (:`Pressed`
    (`self.TestIsGameIsNotOver`
      (:`TRUE`
        (set `self.InputRight` true)
        (`self.JetShake` true)
        (`PrimitiveComponent.AddImpulse` _sphere (* _returnvalue (`self.JetpackBurstForce`)) "None" false)
        (`Timeline|Timeline_3` :!label _label_5
          (:`Update`
            (`PrimitiveComponent.AddImpulse` _sphere _returnvalue "None" false))))))
  (:`Released`
    (`self.TestIsGameIsNotOver`
      (:`TRUE`
        (set `self.InputRight` false)
        (goto _label_5 :!via `Stop`)))))

(event `GameOver`
  (set `self.GameIsOver` true)
  (`PrimitiveComponent.SetLinearDamping` (`self.Sphere`) 999999999.0))

(event `self.ReceiveTick`
  (params (DeltaSeconds :type "Float (single-precision)"))
  (bind _sfx_steam (`self.SFX_Steam`))
  (bind _maxspeedforsoundcue (`self.MaxSpeedForSoundCue`))
  (bind _sfx_steam_2 (`self.SFX_Steam`))
  (`|ExecutionSequence`
    (:`then_0`
      ;[1 1 1] Maj
      (set `self.JetBoost` (or (`self.InputFront`) (`self.InputBack`) (`self.InputLeft`) (`self.InputRight`)))
      ;[1 1 1] Test si première frame de propulsion
      (if (and (`self.JetBoost`) (not (`self.JetBoost_PreviousFrame`)))
        (`GameplayStatics.PlaySound2D` "/Game/TempSounds/pyrostrt_Cue.pyrostrt_Cue")
        (`AudioComponent.Play` _sfx_steam_2 0.0)
        (else
          ;[1 1 1] Si pas de jetpack
          (if (not (`self.JetBoost`))
            (`AudioComponent.Stop` _sfx_steam_2))))
      ;[1 1 1] MAJ pour next frame
      (set `self.JetBoost_PreviousFrame` (`self.JetBoost`)))
    (:`then_1`
      (if (`AudioComponent.IsPlaying` _sfx_steam)
        (bind _returnvalue (`PrimitiveComponent.GetPhysicsLinearVelocity` (`self.Sphere`) "None"))
        (bind _returnvalue_2 (`KismetMathLibrary.VSize` _returnvalue))
        (`AudioComponent.SetPitchMultiplier` _sfx_steam (+ (/ (select `bool` (< _returnvalue_2 20000.0) :`false` _maxspeedforsoundcue :`true` _returnvalue_2) _maxspeedforsoundcue) 0.2))))))

(fn `JetShake`
  (params (LateralShake :type Boolean))
  (`PlayerCameraManager.PlayCameraShake` :`self` (`GameplayStatics.GetPlayerCameraManager` 0) :`ShakeClass` (select `bool` LateralShake :`false` "/Game/CharCaveman/CamShakeX.CamShakeX_C" :`true` "/Game/CharCaveman/CamShakeY.CamShakeY_C" :!type "CameraShake Class Reference") :`Scale` (`KismetMathLibrary.FClamp` (/ (`KismetMathLibrary.VSize` (`SceneComponent.GetComponentVelocity` (`self.Sphere`))) 2000.0) 0.2 2.5)))

(fn `UserConstructionScript`)