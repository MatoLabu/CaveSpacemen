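; Parent Blueprint for fireboxes that can be lit once, each reporting to JetpackGameMode as an inflamed torch with its fireplace size.
; BeginPlay resets actor scale and caches the first child of Visual as the primitive to inflame.
; Inflame sets a guard flag, notifies the game mode, then spawns an enlarged BP_Flame attached at the flame anchor.
; A material swap to M_trunk2 on the cached visual is left disconnected.
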(event `self.ReceiveBeginPlay`
  (bind _asprimitive_component (cast `PrimitiveComponent` (`SceneComponent.GetChildComponent` (`self.Visual`) 0)))
  (set `self.VisualToInflame` _asprimitive_component)
  (`self.SetActorScale3D` (1.0 1.0 1.0)))

(event `Inflame`
  (bind _fireboxflameanchor (`self.FireboxFlameAnchor`))
  (if (not (`self.IsInflamed`))
    (set `self.IsInflamed` true)
    (bind _asjetpack_game_mode (cast `/Game/JetpackGameMode` (`GameplayStatics.GetGameMode`)))
    (`/Game/JetpackGameMode.InflameATorch` _asjetpack_game_mode (`self.SizeOfFireplace`))
    ;[1 1 1] Spawn flames
    (bind _returnvalue (`|SpawnActorFromClass` "/Game/Fireboxes/BP_Flame.BP_Flame_C" (`SceneComponent.K2_GetComponentToWorld` _fireboxflameanchor) "Undefined" "OverrideRootScale"))
    (`self.SetActorScale3D` _returnvalue (5.0 5.0 5.0))
    (`self.K2_AttachToComponent` _returnvalue _fireboxflameanchor "None" "KeepWorld" "KeepWorld" "KeepRelative" true)))

(fn `UserConstructionScript`)