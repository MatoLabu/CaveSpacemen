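; BP_Flame is a flame actor whose graph is built to tumble four fire components: Fire1, Fire1b, Fire2 and Fire2b.
; Two self-restarting timelines each rotate a pair through full turns on differing axes, with a random length per cycle to vary the motion.
; No event triggers either loop, so the animation never runs as wired, and the construction script is empty.
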(fn `UserConstructionScript`)